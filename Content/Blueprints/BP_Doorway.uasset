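; BP_Doorway is an always-interactable doorway that ends the game with a win when used.
; OnInteract pauses the game, disables player input, shows the cursor, hides BP_HUD's player widget and displays WBP_YouWinScreen.
; A timeline-driven door toggle, which picks a swing direction by dot product, remains in the graph but is disconnected and never runs.
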(event `/Game/Blueprints/Interfaces/BPI_Interact.OnInteract`
  (params (InteractingPlayer :type "Character Object Reference"))
  (bind _returnvalue (`GameplayStatics.GetPlayerController` 0))
  ;[1 1 1] Door
  ;;[1 1 1] Win Screen/End
  (`GameplayStatics.SetGamePaused` true)
  (`self.DisableInput` _returnvalue)
  (set `PlayerController.bShowMouseCursor` true _returnvalue)
  (bind _asbp_hud (cast `/Game/Blueprints/BP_HUD` (`PlayerController.GetHUD` _returnvalue)))
  (`Widget.SetVisibility` (`/Game/Blueprints/BP_HUD.PlayerHUD` _asbp_hud) "Hidden")
  (bind _returnvalue_2 (`|CreateWidget` "/Game/Blueprints/WidgetBlueprints/WBP_YouWinScreen.WBP_YouWinScreen_C"))
  (bind _output_get (set `self.YouWinScreen` _returnvalue_2))
  (`UserWidget.AddToPlayerScreen` _output_get 0))

(fn `IsInteractable`
  (returns (Interactable :type Boolean))
  (return true))

(fn `UserConstructionScript`)