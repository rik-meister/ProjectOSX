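; BPC_Health is a health component that tracks current health, healing and death for its owner.
; TakingDamage subtracts damage without clamping, prints the new value and calls Dead at zero or below.
; GainingHealth clamps healing between zero and MaxHealth, or calls Dead again if already dead.
; Dead uses a DoOnce to set the Dead flag and call the GeneralDeath dispatcher.
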(fn `Dead`
  (`/Engine/EditorBlueprintResources/StandardMacros.DoOnce` false
    (:`Completed`
      (set `self.Dead?` true)
      (`self.GeneralDeath`))))

(fn `GainingHealth`
  (params (GainingHealth :type Integer))
  (if (`self.Dead?`)
    (`self.Dead`)
    (else
      (set `self.CurrentHealth` (`KismetMathLibrary.Clamp` (+ GainingHealth (`self.CurrentHealth`)) 0 (`self.MaxHealth`))))))

(fn `TakingDamage`
  (params (IncomingDamage :type Integer))
  (bind _output_get (set `self.CurrentHealth` (- (`self.CurrentHealth`) IncomingDamage)))
  (`KismetSystemLibrary.PrintString` (`KismetStringLibrary.Conv_IntToString` _output_get))
  (if (<= _output_get 0)
    (`self.Dead`)
    (else
      (return))))