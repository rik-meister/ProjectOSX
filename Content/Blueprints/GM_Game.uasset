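; GM_Game is a game mode Blueprint that scatters crates across randomly chosen spawn points when play begins.
; SpawnCrate gathers every BP_CrateSpawnPoint actor, then repeatedly picks one at random and spawns a BP_Crate at its location with default rotation and scale.
; Each used point is removed from the local array and destroyed, so a fixed number of crates spawn without sharing a point.
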(event `self.ReceiveBeginPlay`
  (`self.SpawnCrate`))

(fn `SpawnCrate`
  (locals (CrateLocalSpawnRef :type "Array of /Game/Blueprints/BP_CrateSpawnPoint Object Reference") (LocalItem :type "/Game/Blueprints/BP_CrateSpawnPoint Object Reference"))
  (bind _outactors (`GameplayStatics.GetAllActorsOfClass` "/Game/Blueprints/BP_CrateSpawnPoint.BP_CrateSpawnPoint_C"))
  (set `local.CrateLocalSpawnRef` _outactors)
  (for _ (range 5)
    (set `local.LocalItem` (`KismetArrayLibrary.Array_Random` (`local.CrateLocalSpawnRef`)))
    (`|SpawnActorFromClass` "/Game/Blueprints/BP_Crate.BP_Crate_C" (`KismetMathLibrary.MakeTransform` (`self.K2_GetActorLocation` (`local.LocalItem`))) "AdjustIfPossibleButAlwaysSpawn" "MultiplyWithRoot" null null)
    ;[1 1 1] Makes sure Crate does not spawn in same location
    (`KismetArrayLibrary.Array_RemoveItem` (`local.CrateLocalSpawnRef`) (`local.LocalItem`))
    (`self.K2_DestroyActor` (`local.LocalItem`))))

(fn `UserConstructionScript`)