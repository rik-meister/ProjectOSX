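; Player state that tracks the player's score with a time-windowed combo multiplier.
; AddPoints updates the combo, adds the incoming points times the multiplier, and broadcasts the new score.
; Each call within the combo window increments the multiplier, otherwise it restarts at one.
; A timer restarted on every pickup resets the combo when the window expires, with combo changes broadcast through an event dispatcher.
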(fn `AddPoints`
  (params (PointsToAdd :type Integer))
  (`self.UpdateCombo` 0)
  (bind _output_get (set `self.CurrentPoints` (+ (* PointsToAdd (`self.ComboMultiplier`)) (`self.CurrentPoints`))))
  (`self.OnScoreChange` _output_get))

(fn `GetPoints`
  (returns (ReturnValue :type Integer))
  (return (`self.CurrentPoints`)))

(fn `ResetCombo`
  (bind _output_get (set `self.ComboMultiplier` 1))
  (`self.OnComboChange` _output_get))

(fn `UpdateCombo`
  (params (PointsToMultiply :type Integer))
  (bind _returnvalue (`KismetSystemLibrary.GetGameTimeInSeconds`))
  (if (< (- _returnvalue (`self.LastPickupTime`)) (`self.ComboWindow`))
    (bind _result (`/Engine/EditorBlueprintResources/StandardMacros.IncrementInt` (`self.ComboMultiplier`))
      (:`  `
        (`self.OnComboChange` _result)))
    (else
      (bind _output_get (set `self.ComboMultiplier` 1))
      (`self.OnComboChange` _output_get)))
  (set `self.LastPickupTime` _returnvalue)
  (`KismetSystemLibrary.K2_ClearAndInvalidateTimerHandle` (`self.ComboResetTimer`))
  (bind _returnvalue_2 (`KismetSystemLibrary.K2_SetTimer` null "ResetCombo" (`self.ComboWindow`)))
  (set `self.ComboResetTimer` _returnvalue_2))

(fn `UserConstructionScript`)